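; Player character Blueprint that changes the camera spring arm length while the player sprints.
; BeginPlay caches the arm's default length as the blend origin.
; Sprint start plays a timeline that lerps the arm from that default to the sprint length, and sprint end reverses the same timeline to ease it back.
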(event EventOnSprintStart
  (bind _newtrack_0 (Timeline|SpringArm%20sprint%20timeline Play)
    (:Update
      (Variables|/Script/Engine.SpringArmComponent|SetTargetArmLength (Variables|Default|GetSpringArmComponent) (Math|Float|Lerp (Variables|SprintSettings|GetDefaultArmLenth) (Variables|SprintSettings|GetSprintArmLength) _newtrack_0)))))

(event EventOnSprintEnd
  (bind _newtrack_0 (Timeline|SpringArm%20sprint%20timeline Reverse)
    (:Update
      (Variables|/Script/Engine.SpringArmComponent|SetTargetArmLength (Variables|Default|GetSpringArmComponent) (Math|Float|Lerp (Variables|SprintSettings|GetDefaultArmLenth) (Variables|SprintSettings|GetSprintArmLength) _newtrack_0)))))

(event EventBeginPlay
  (Variables|SprintSettings|SetDefaultArmLenth (Variables|/Script/Engine.SpringArmComponent|GetTargetArmLength (Variables|Default|GetSpringArmComponent))))

(fn ConstructionScript)