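; Pawn Blueprint for the T-72B tank vehicle, setting up collision that follows its gun and turret.
; On BeginPlay it attaches MuzzleCollision and TurretCollision to the gun and turret joints of the skeletal mesh, then adjusts their relative offsets.
; The graph holds no other active logic, as overlap, Tick and the construction script are empty.
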(event EventBeginPlay
  (bind _skeletalmesh (Variables|Default|GetSkeletalMesh))
  (bind _turretcollision (Variables|Default|GetTurretCollision))
  (bind _relativelocation (Variables|/Script/Engine.SceneComponent|GetRelativeLocation _turretcollision))
  (Transformation|AttachComponentToComponent (Variables|Default|GetMuzzleCollision) _skeletalmesh "gun_jnt" "KeepRelative" "KeepRelative" "KeepRelative" true)
  (Transformation|AttachComponentToComponent (Variables|Default|GetTurretCollision) _skeletalmesh "turret_jnt" "KeepRelative" "KeepRelative" "KeepRelative" true)
  (Transformation|SetRelativeLocation (Variables|Default|GetTurretCollision) (Math|Vector|MakeVector (.x _relativelocation) (.y _relativelocation) 23.0) false false)
  (Transformation|SetRelativeLocation (Variables|Default|GetMuzzleCollision) (Math|Vector|MakeVector 2.9e+02 (.y (Variables|/Script/Engine.SceneComponent|GetRelativeLocation (Variables|Default|GetMuzzleCollision))) 6.0) false false))

(event Collision|EventActorBeginOverlap
  (params (OtherActor :type Actor%20Object%20Reference)))

(event EventTick
  (params (DeltaSeconds :type Float%20%28single-precision%29)))

(fn ConstructionScript)