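; Showcase Blueprint for the East IMV Tigr-M vehicle, exposing its moving parts, skin and effects to adjustable controls.
; Generic slider, twin-slider, button and checkbox events each forward their value to a setter for doors, hatch, wheels, turret, gun, wipers, lights, skin, damage or firing FX.
; The construction script calls the parent's, then creates a dynamic material instance on the skeletal mesh's first material slot.
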(event EventSetSliderVariable5
  (params (NewValue :type Float%20%28double-precision%29))
  (CallFunction|SetWindowCleanersAngle NewValue))

(event EventSetSliderVariable6
  (params (NewValue :type Float%20%28double-precision%29))
  (CallFunction|SetLightsEmissivity NewValue))

(event EventSetCheckboxVariable0
  (params (NewState :type Boolean))
  (CallFunction|SetShowDamaged NewState))

(event EventSetButtonsVariable0
  (params (NewIndex :type Integer))
  (CallFunction|SetSkinType (Math|Conversions|ToFloat(Integer) NewIndex)))

(event EventSetCheckboxVariable1
  (params (NewState :type Boolean))
  (CallFunction|SetActivateFiring NewState))

(event EventSetTwinSliderVariable0
  (params (bFirstSlider? :type Boolean) (NewFirstValue :type Float%20%28double-precision%29) (NewSecondValue :type Float%20%28double-precision%29))
  (CallFunction|SetFrontDoorsAngle NewFirstValue NewSecondValue))

(event EventSetTwinSliderVariable1
  (params (bFirstSlider? :type Boolean) (NewFirstValue :type Float%20%28double-precision%29) (NewSecondValue :type Float%20%28double-precision%29))
  (CallFunction|SetRearDoorsAngle NewFirstValue NewSecondValue))

(event EventSetSliderVariable0
  (params (NewValue :type Float%20%28double-precision%29))
  (CallFunction|SetRoofHatchAngle NewValue))

(event EventSetSliderVariable1
  (params (NewValue :type Float%20%28double-precision%29))
  (CallFunction|SetTurretRotation NewValue))

(event EventSetSliderVariable2
  (params (NewValue :type Float%20%28double-precision%29))
  (CallFunction|SetGunElevation NewValue))

(event EventSetSliderVariable3
  (params (NewValue :type Float%20%28double-precision%29))
  (CallFunction|SetWheelSpeed NewValue))

(event EventSetSliderVariable4
  (params (NewValue :type Float%20%28double-precision%29))
  (CallFunction|SetFrontWheelsAngle NewValue))

(fn ConstructionScript
  (|CallParentFunction)
  (Rendering|Material|CreateDynamicMaterialInstance (Variables|Default|GetSkeletalMesh) 0 0 "None" :!class /Script/Engine.PrimitiveComponent))