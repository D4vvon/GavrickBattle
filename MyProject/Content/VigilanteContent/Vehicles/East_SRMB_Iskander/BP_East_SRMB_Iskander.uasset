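; Vehicle Blueprint for the East Iskander missile launcher, exposing events that control its articulation, appearance and effects.
; Setters write wheel, cockpit door, cargo, cargo door and holder values to the cached Anim Blueprint, and wheel speed also toggles wheel and dust-trail VFX.
; Dynamic body and cargo materials created in the Construction Script take skin type, with light emissivity on the body.
; Damage display swaps visibility between the skeletal mesh and damaged model.
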(event Custom|SetWheelVFX
  (params (Speed :type Float%20%28double-precision%29))
  ;[1 1 1] Set wheel vfx
  (Components|Activation|SetActive (Variables|Default|GetWheelVFX_Rtf) (> Speed 0.0) false))

(event Custom|SetSkinType
  (params (SkinType :type Float%20%28double-precision%29))
  ;[1 1 1] Set skin type
  (Rendering|Material|SetScalarParameterValue (Variables|Default|GetBodyMaterial) "SkinType" SkinType :!class /Script/Engine.MaterialInstanceDynamic)
  (Rendering|Material|SetScalarParameterValue (Variables|Default|GetCargoMaterial) "SkinType" SkinType :!class /Script/Engine.MaterialInstanceDynamic))

(event Custom|SetLightsEmissivity
  (params (Emissivity :type Float%20%28double-precision%29))
  ;[1 1 1] Set lights emissivity
  (Rendering|Material|SetScalarParameterValue (Variables|Default|GetBodyMaterial) "EmissiveMultiplier" Emissivity :!class /Script/Engine.MaterialInstanceDynamic))

(event Custom|SetDamagedModel
  (params (ShowDamage :type Boolean))
  ;[1 1 1] Set damaged vehicle
  (Rendering|SetVisibility (Variables|Default|GetSkeletalMesh) (not ShowDamage) true)
  (Rendering|SetVisibility (Variables|Default|GetDamageVehicle) ShowDamage true))

(event Custom|SetWheelSpeed
  (params (Speed :type Float%20%28double-precision%29))
  ;[1 1 1] Set wheel speed
  (bind _output_get (Variables|/Game/VigilanteContent/Vehicles/East_SRMB_Iskander/ABP_East_SRMB_Iskander.ABP_East_SRMB_Iskander_C|SetWheelSpeed (Variables|Default|GetAnimInstance) Speed))
  (CallFunction|SetWheelVFX _output_get))

(event Custom|SetWheelAngle
  (params (Angle :type Float%20%28double-precision%29))
  ;[1 1 1] Set wheel angle
  (Variables|/Game/VigilanteContent/Vehicles/East_SRMB_Iskander/ABP_East_SRMB_Iskander.ABP_East_SRMB_Iskander_C|SetWheelAngle (Variables|Default|GetAnimInstance) Angle))

(event Custom|SetCockpitDoorAngle
  (params (Angle :type Float%20%28double-precision%29))
  ;[1 1 1] Set cockpit door angles
  (Variables|/Game/VigilanteContent/Vehicles/East_SRMB_Iskander/ABP_East_SRMB_Iskander.ABP_East_SRMB_Iskander_C|SetCockPitDoorAngle (Variables|Default|GetAnimInstance) Angle))

(event Custom|SetHolderHeight
  (params (Height :type Float%20%28double-precision%29))
  ;[1 1 1] Set holder height
  (Variables|/Game/VigilanteContent/Vehicles/East_SRMB_Iskander/ABP_East_SRMB_Iskander.ABP_East_SRMB_Iskander_C|SetHolderHeight (Variables|Default|GetAnimInstance) Height))

(event Custom|SetCargoDoorAngles
  (params (Value :type Float%20%28double-precision%29))
  (bind _animinstance (Variables|Default|GetAnimInstance))
  ;[1 1 1] Set cargo door angles
  (Variables|/Game/VigilanteContent/Vehicles/East_SRMB_Iskander/ABP_East_SRMB_Iskander.ABP_East_SRMB_Iskander_C|SetCargoDoorAngle _animinstance (Math|Float|MapRangeClamped Value 0.0 1.0 0.0 1.2e+02))
  (Variables|/Game/VigilanteContent/Vehicles/East_SRMB_Iskander/ABP_East_SRMB_Iskander.ABP_East_SRMB_Iskander_C|SetBackDoorAngle _animinstance (Math|Float|MapRangeClamped Value 0.0 1.0 0.0 7e+01)))

(event Custom|SetCargoAngle
  (params (Angle :type Float%20%28double-precision%29))
  ;[1 1 1] Set cargo angle
  (Variables|/Game/VigilanteContent/Vehicles/East_SRMB_Iskander/ABP_East_SRMB_Iskander.ABP_East_SRMB_Iskander_C|SetCargoAngle (Variables|Default|GetAnimInstance) Angle))

(event EventBeginPlay
  (|CallParentFunction)
  (bind _asabp_east_srmb_iskander (Utilities|Casting|CastToABP_East_SRMB_Iskander (Components|SkeletalMesh|GetAnimInstance (Variables|Default|GetSkeletalMesh))))
  (Variables|Default|SetAnimInstance _asabp_east_srmb_iskander))

(fn ConstructionScript
  (bind _skeletalmesh (Variables|Default|GetSkeletalMesh))
  (bind _returnvalue (Rendering|Material|CreateDynamicMaterialInstance _skeletalmesh 3 0 "None" :!class /Script/Engine.PrimitiveComponent))
  (Variables|Default|SetBodyMaterial _returnvalue)
  (bind _returnvalue_2 (Rendering|Material|CreateDynamicMaterialInstance _skeletalmesh 1 0 "None" :!class /Script/Engine.PrimitiveComponent))
  (Variables|Default|SetCargoMaterial _returnvalue_2))