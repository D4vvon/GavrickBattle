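; Showcase Blueprint for the East SRMB Iskander missile vehicle, exposing its visual and articulation settings to generic slider, checkbox and button controls.
; Numbered slider events forward values to setters for wheel speed and angle, cockpit and cargo doors, cargo angle, holder height and light emissivity.
; A checkbox toggles the damaged model, and a button index, converted to float, selects the skin.
; The construction script only calls its parent.
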(event EventBeginPlay
  (|CallParentFunction) ; This node is disabled and will not be called.\nDrag off pins to build functionality.
)

(event Collision|EventActorBeginOverlap
  (params (OtherActor :type Actor%20Object%20Reference))
  (|CallParentFunction OtherActor) ; This node is disabled and will not be called.\nDrag off pins to build functionality.
)

(event EventSetSliderVariable5
  (params (NewValue :type Float%20%28double-precision%29))
  ;[1 1 1] Sliders
  (CallFunction|SetCargoDoorAngles NewValue))

(event EventSetSliderVariable6
  (params (NewValue :type Float%20%28double-precision%29))
  ;[1 1 1] Sliders
  (CallFunction|SetCargoAngle NewValue))

(event EventTick
  (params (DeltaSeconds :type Float%20%28single-precision%29))
  (|CallParentFunction DeltaSeconds) ; This node is disabled and will not be called.\nDrag off pins to build functionality.
)

(event EventSetSliderVariable0
  (params (NewValue :type Float%20%28double-precision%29))
  ;[1 1 1] Sliders
  (CallFunction|SetWheelSpeed NewValue))

(event EventSetSliderVariable1
  (params (NewValue :type Float%20%28double-precision%29))
  ;[1 1 1] Sliders
  (CallFunction|SetWheelAngle NewValue))

(event EventSetSliderVariable2
  (params (NewValue :type Float%20%28double-precision%29))
  ;[1 1 1] Sliders
  (CallFunction|SetCockpitDoorAngle NewValue))

(event EventSetSliderVariable3
  (params (NewValue :type Float%20%28double-precision%29))
  ;[1 1 1] Sliders
  (CallFunction|SetLightsEmissivity NewValue))

(event EventSetCheckboxVariable0
  (params (NewState :type Boolean))
  ;[1 1 1] Checkboxes
  (CallFunction|SetDamagedModel NewState))

(event EventSetSliderVariable4
  (params (NewValue :type Float%20%28double-precision%29))
  ;[1 1 1] Sliders
  (CallFunction|SetHolderHeight NewValue))

(event EventSetButtonsVariable0
  (params (NewIndex :type Integer))
  ;[1 1 1] Buttons
  (CallFunction|SetSkinType (Math|Conversions|ToFloat(Integer) NewIndex)))

(fn ConstructionScript
  (|CallParentFunction))