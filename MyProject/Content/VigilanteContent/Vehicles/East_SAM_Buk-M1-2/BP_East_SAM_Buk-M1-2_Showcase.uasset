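; Showcase Blueprint for the East SAM Buk-M1-2 vehicle, exposing its adjustable features to slider, button and checkbox input.
; Each input event forwards its value to a setter for speed, skin type, launcher elevation, damaged-model visibility, light emissivity, hatch rotation or turret rotation.
; The setters are not defined in this graph, and the construction script only calls the parent's.
; The event commented as platform rotation actually sets light emissivity.
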(event EventSetSliderVariable2
  (params (NewValue :type Float%20%28double-precision%29))
  ;[1 1 1] Set Platform rotation
  (CallFunction|SetLightsEmissivity NewValue))

(event EventSetSliderVariable3
  (params (NewValue :type Float%20%28double-precision%29))
  ;[1 1 1] Set hatches rotation
  (CallFunction|SetHatchesRotation NewValue))

(event EventSetCheckboxVariable0
  (params (NewState :type Boolean))
  ;[1 1 1] Damaged model visibility
  (CallFunction|SetShowDamaged NewState))

(event EventSetSliderVariable4
  (params (NewValue :type Float%20%28double-precision%29))
  ;[1 1 1] Turret rotation
  (CallFunction|SetTurretRotation NewValue))

(event EventSetSliderVariable0
  (params (NewValue :type Float%20%28double-precision%29))
  ;[1 1 1] Speed
  (CallFunction|SetSpeed NewValue))

(event EventSetSliderVariable1
  (params (NewValue :type Float%20%28double-precision%29))
  ;[1 1 1] Launcher elevation
  (CallFunction|LauncherElevation NewValue))

(event EventSetButtonsVariable0
  (params (NewIndex :type Integer))
  ;[1 1 1] Skin variant
  (CallFunction|SetSkinType (Math|Conversions|ToFloat(Integer) NewIndex)))

(fn ConstructionScript
  (|CallParentFunction))