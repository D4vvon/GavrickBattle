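; Showcase variant of the West M1133 Medic vehicle Blueprint that exposes its adjustable features to generic showcase controls.
; Indexed slider, checkbox and button events forward values to setters for wheels, mirrors, hatch, turret, gun elevation and light emissivity.
; Checkboxes toggle damage display and firing, while the button index is converted to a float to select the skin.
; The construction script only calls its parent.
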(event EventSetSliderVariable1
  (params (NewValue :type Float%20%28double-precision%29))
  ;[1 1 1] Showcase float controls
  (CallFunction|SetFrontWheelsAngle NewValue))

(event EventSetCheckboxVariable0
  (params (NewState :type Boolean))
  ;[1 1 1] Showcase checkbox controls
  (CallFunction|SetShowDamaged NewState))

(event EventSetCheckboxVariable1
  (params (NewState :type Boolean))
  ;[1 1 1] Showcase checkbox controls
  (CallFunction|SetActivateFiring NewState))

(event EventSetButtonsVariable0
  (params (NewIndex :type Integer))
  ;[1 1 1] Checkbox button controls
  (CallFunction|SetSkinType (Math|Conversions|ToFloat(Integer) NewIndex)))

(event EventSetSliderVariable2
  (params (NewValue :type Float%20%28double-precision%29))
  ;[1 1 1] Showcase float controls
  (CallFunction|SetMirrorsAngle NewValue))

(event EventSetSliderVariable3
  (params (NewValue :type Float%20%28double-precision%29))
  ;[1 1 1] Showcase float controls
  (CallFunction|SetHatchAngle NewValue))

(event EventSetSliderVariable4
  (params (NewValue :type Float%20%28double-precision%29))
  ;[1 1 1] Showcase float controls
  (CallFunction|SetTurretAngle NewValue))

(event EventSetSliderVariable5
  (params (NewValue :type Float%20%28double-precision%29))
  ;[1 1 1] Showcase float controls
  (CallFunction|SetGunElevation NewValue))

(event EventSetSliderVariable6
  (params (NewValue :type Float%20%28double-precision%29))
  ;[1 1 1] Showcase float controls
  (CallFunction|SetLightsEmissivity NewValue))

(event EventSetSliderVariable0
  (params (NewValue :type Float%20%28double-precision%29))
  ;[1 1 1] Showcase float controls
  (CallFunction|SetWheelSpeed NewValue))

(fn ConstructionScript
  (|CallParentFunction))